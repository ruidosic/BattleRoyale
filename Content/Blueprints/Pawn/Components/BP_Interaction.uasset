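; Interaction component for BP_CharacterPawn that picks a target actor and tracks the character's interaction state.
; It caches the owning pawn on BeginPlay and passes interaction flag changes to the character's AnimBP via a message.
; SelectNearestTarget compares horizontal distance only, ignoring height, and returns the closest actor within a fixed range.
; TargetDamage, which requests rotation toward a valid target, is unfinished and never called in the event graph.
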(event `self.ReceiveBeginPlay`
  ;[1 1 1] Set Character Variable
  (bind _asbp_character_pawn (cast `/Game/Blueprints/Pawn/BP_CharacterPawn` (`self.GetOwner`)))
  (set `self.Character` _asbp_character_pawn))

(fn `SelectNearestTarget`
  (params (TargetArray :type "Array of Actor Object Reference"))
  (returns (Target :type "Actor Object Reference"))
  (bind (_returnvalue_x _returnvalue_y _returnvalue_z) (`KismetMathLibrary.BreakVector` (`Actor.K2_GetActorLocation` (`self.Character`))))
  (if (> (`KismetArrayLibrary.Array_LastIndex` TargetArray) 0)
    (set `self.NearestDistance` 5000.0)
    (for _array_element TargetArray
      (bind (_returnvalue_x_2 _returnvalue_y_2) (`KismetMathLibrary.BreakVector` (`Actor.K2_GetActorLocation` _array_element)))
      (bind _returnvalue (`KismetMathLibrary.VSize` (- (`KismetMathLibrary.MakeVector` _returnvalue_x_2 _returnvalue_y_2 _returnvalue_z) (`KismetMathLibrary.MakeVector` _returnvalue_x _returnvalue_y _returnvalue_z))))
      (if (< _returnvalue (`self.NearestDistance`))
        (set `self.NearestDistance` _returnvalue)
        (set `self.Target` _array_element)))
    (return (`self.Target`))
    (else
      (bind _output_get (set `self.Target` (`|GetArrayItem` TargetArray)))
      (return _output_get))))

(fn `SetIsInteraction`
  (params (IsInteraction :type Boolean))
  (bind _output_get (set `self.IsInteraction` IsInteraction))
  ;[1 1 1] Send to AnimBP
  (message `/Game/Blueprints/Pawn/BPI_AnimInterface.Set_IsInteraction` (`self.CharacterAnimBP`) _output_get))