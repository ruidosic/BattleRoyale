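; Character weapon actor, configured by WeaponStruct, that handles firing effects, bullets, noise and damage.
; Shoot, whose firing path runs only for player 0's pawn, spawns BP_BulletProjectile or line-traces along the owner's aim within a random spread cone.
; Both modes feed BulletHit, which applies surface-based particles, decals and sounds, point damage and physics impulses.
; Each bullet widens spread, which a looping timer eases back until a retriggerable delay resets it.
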(event `CharacterWeaponSet`
  ;[1 1 1] Set Weapon
  (message `/Game/Blueprints/Weapon/BP_WeaponInterface.SetWeapon` (`self.GetOwner`) self))

(event `self.ReceiveBeginPlay`
  ;[1 1 1] Set Owner (Begin Play)
  (set `self.OwnerCharacter` (`self.GetOwner`)))

(event `Shoot`
  (bind (_start _end) (`self.BulletDirection`))
  (bind ((`Damage_8_93B86D544DB6A894C92897AA97600886` _damage) (`BulletProjectile_11_D028639C414079989764CC9B1A28F9A4` _bulletprojectile)) (break `/Game/Blueprints/Weapon/Structures/Struct_Weapon/Struct_Weapon` (`self.WeaponStruct`)))
  (bind _returnvalue_location (`KismetMathLibrary.BreakTransform` (`SceneComponent.GetSocketTransform` (`self.CharacterWeaponMesh`) "Socket_Muzzle" "RTS_World")))
  (bind (_returnvalue_location_2 _returnvalue_rotation) (`KismetMathLibrary.BreakTransform` (`SceneComponent.GetSocketTransform` (`self.CharacterWeaponMesh`) (`self.MuzzleSocket`) "RTS_World")))
  (bind (_returnvalue_location_3 _returnvalue_rotation_2) (`KismetMathLibrary.BreakTransform` (`SceneComponent.GetSocketTransform` (`self.CharacterWeaponMesh`) (`self.MuzzleSocket`) "RTS_World")))
  (bind ((`Bullet_Min_15_63FC76DA40FF1A0AC334AFBB37AAC0B5` _bullet_min) (`Bullet_Max_14_20A4940548C029B10CDEC085890CF03D` _bullet_max) (`RandomNumBullets_5_CECE948140E421EAE1692899D7C3536C` _randomnumbullets)) (break `/Game/Blueprints/Weapon/Structures/Struct_Weapon/Struct_Weapon_RapidlyOfFire` (`.RapidlyOfFire_27_4DB41EBC4E02B3365DE5A8835C957E41` (break `/Game/Blueprints/Weapon/Structures/Struct_Weapon/Struct_Weapon` (`self.WeaponStruct`)))))
  (bind (_recoil_min _recoil_max) (break `/Game/Blueprints/Weapon/Structures/Struct_Weapon/Struct_Weapon_Spreading` (`.Spreading_21_99892FAD48D8FDC516D29698A779D626` (break `/Game/Blueprints/Weapon/Structures/Struct_Weapon/Struct_Weapon` (`self.WeaponStruct`)))))
  ;[1 1 1] Shoot Animation Select
  (if (== (`self.Ammo_InClip`) 0)
    (`SkeletalMeshComponent.PlayAnimation` (`self.CharacterWeaponMesh`) (`.AnimationEmpty_32_3252DDAA4184CB386AE75F90C0035004` (break `/Game/Blueprints/Weapon/Structures/Struct_Weapon/Struct_Weapon_Visual` (`.Visual_18_5CE5B0BA437651B375F8FFB7652EC144` (break `/Game/Blueprints/Weapon/Structures/Struct_Weapon/Struct_Weapon` (`self.WeaponStruct`))))) false)
    (`self.OnEmptyShoot`)
    ;[1 1 1] Camera Shake
    (if (== (`self.OwnerCharacter`) (`GameplayStatics.GetPlayerPawn` 0))
      (`PlayerCameraManager.PlayCameraShake` :`self` (`PlayerController.PlayerCameraManager` (`GameplayStatics.GetPlayerController` 0)) :`ShakeClass` (`.CameraShakeClass_15_E4CD03A24482E59EFB8F6FB20C2E62B5` (break `/Game/Blueprints/Weapon/Structures/Struct_Weapon/Struct_Weapon_Spreading` (`.Spreading_21_99892FAD48D8FDC516D29698A779D626` (break `/Game/Blueprints/Weapon/Structures/Struct_Weapon/Struct_Weapon` (`self.WeaponStruct`))))) :`Scale` (`KismetMathLibrary.FClamp` (+ (`self.Degrees`) _recoil_min) 0.0 _recoil_max))
      ;[1 1 1] Muzzle
      (`GameplayStatics.SpawnEmitterAttached` (`.MuzzleParticle_16_6B7B8AAE4733D2181BBAE882946C0C81` (break `/Game/Blueprints/Weapon/Structures/Struct_Weapon/Struct_Weapon_Visual` (`.Visual_18_5CE5B0BA437651B375F8FFB7652EC144` (break `/Game/Blueprints/Weapon/Structures/Struct_Weapon/Struct_Weapon` (`self.WeaponStruct`))))) (`self.CharacterWeaponMesh`) "Socket_Muzzle")
      ;[1 1 1] Shoot Sound
      (`GameplayStatics.PlaySoundAtLocation` (`.ShootSound_19_EDEB10A84A9F15EA6D3B498A71BE5855` (break `/Game/Blueprints/Weapon/Structures/Struct_Weapon/Struct_Weapon_Visual` (`.Visual_18_5CE5B0BA437651B375F8FFB7652EC144` (break `/Game/Blueprints/Weapon/Structures/Struct_Weapon/Struct_Weapon` (`self.WeaponStruct`))))) _returnvalue_location (struct) 1.0 1.0 0.0 null null null)
      ;[1 1 1] Shoot Noise
      (message `/Game/Blueprints/Weapon/BP_WeaponInterface.WeaponMakeNoise` (`self.OwnerCharacter`) (`.ShootLoudness_10_4BDE3D984D7B17CC58BD2C84107DB571` (break `/Game/Blueprints/Weapon/Structures/Struct_Weapon/Struct_Weapon_RapidlyOfFire` (`.RapidlyOfFire_27_4DB41EBC4E02B3365DE5A8835C957E41` (break `/Game/Blueprints/Weapon/Structures/Struct_Weapon/Struct_Weapon` (`self.WeaponStruct`))))) (`SceneComponent.K2_GetComponentLocation` (`self.CharacterWeaponMesh`)) (`self.OwnerCharacter`))
      ;[1 1 1] Bullet
      (if _randomnumbullets
        (for _ (range _bullet_min (+ (`KismetMathLibrary.RandomIntegerInRange` _bullet_min _bullet_max) 1))
          (if (`.UseBulletProjectile_1_63FC76DA40FF1A0AC334AFBB37AAC0B5` (break `/Game/Blueprints/Weapon/Structures/Struct_Weapon/Struct_Weapon_Bullet` (`.BulletProjectile_11_D028639C414079989764CC9B1A28F9A4` (break `/Game/Blueprints/Weapon/Structures/Struct_Weapon/Struct_Weapon` (`self.WeaponStruct`))))) :!label _label
            ;[1 1 1] Spawn Projectile Bullet
            (bind (_outhit _returnvalue) (`KismetSystemLibrary.LineTraceSingleForObjects` _start _end (`|MakeArray` "ObjectTypeQuery1" "ObjectTypeQuery2" "ObjectTypeQuery4" "ObjectTypeQuery5" "ObjectTypeQuery8" "ObjectTypeQuery9" "ObjectTypeQuery6" "ObjectTypeQuery3" :!type "EObjectTypeQuery Enum") true (`|MakeArray` (`self.OwnerCharacter`))))
            (bind _bulletstartlocation (`self.CheckWeaponCollision` _returnvalue_location_3 _returnvalue_rotation_2))
            (bind _returnvalue_2 (`|SpawnActorFromClass` "/Game/Blueprints/Weapon/BP_BulletProjectile.BP_BulletProjectile_C" (`KismetMathLibrary.MakeTransform` _bulletstartlocation _returnvalue_rotation_2) "AlwaysSpawn" "OverrideRootScale" null (`KismetMathLibrary.Normal` (- _returnvalue_location_3 (+ (select `bool` _returnvalue :`false` (`.End` (`self.BulletDirection`)) :`true` (`.Location` (`GameplayStatics.BreakHitResult` _outhit))) (* (`KismetMathLibrary.Conv_RotatorToVector` _returnvalue_rotation_2) -80.0)))) _bulletprojectile (`.BaseDamage_8_63FC76DA40FF1A0AC334AFBB37AAC0B5` (break `/Game/Blueprints/Weapon/Structures/Struct_Weapon/Struct_Weapon_Damage` _damage)) null))
            (`self.SpreadingDecrease`)
            (add `/Game/Blueprints/Weapon/BP_BulletProjectile.BulletHit` _returnvalue_2 (delegate `BulletHit`))
            (else
              (`self.BulletTrace` _returnvalue_location_2 _returnvalue_rotation))))
        (else
          (for _ (range _bullet_min (+ _bullet_max 1))
            (goto _label)))))))

(event `BulletHit`
  (params (Hit :type "HitResult Structure") (`DamageUpdate(ric)` :type "Float (double-precision)"))
  (bind (_bblockinghit _binitialoverlap _time _distance _location _impactpoint _normal _impactnormal _physmat _hitactor _hitcomponent _hitbonename) (`GameplayStatics.BreakHitResult` Hit))
  (bind ((`Damage_8_93B86D544DB6A894C92897AA97600886` _damage) (`BulletProjectile_11_D028639C414079989764CC9B1A28F9A4` _bulletprojectile)) (break `/Game/Blueprints/Weapon/Structures/Struct_Weapon/Struct_Weapon` (`self.WeaponStruct`)))
  (bind _returnvalue (`KismetMathLibrary.Conv_VectorToRotator` _normal))
  (bind ((`DamageType_17_BD173512406557695A31A1AADF8FE0E7` _damagetype)) (break `/Game/Blueprints/Weapon/Structures/Struct_Weapon/Struct_Weapon_Damage` (`.Damage_8_93B86D544DB6A894C92897AA97600886` (break `/Game/Blueprints/Weapon/Structures/Struct_Weapon/Struct_Weapon` (`self.WeaponStruct`)))))
  (bind ((`BaseDamage_8_63FC76DA40FF1A0AC334AFBB37AAC0B5` _basedamage) (`DamageType_17_BD173512406557695A31A1AADF8FE0E7` _damagetype_2)) (break `/Game/Blueprints/Weapon/Structures/Struct_Weapon/Struct_Weapon_Damage` _damage))
  (bind (_particle _decal _decalsize _decalrotation _soundhit) (`self.SelectSurfaceType` (`PhysicalMaterial.SurfaceType` _physmat) _returnvalue))
  (bind _returnvalue_2 (`KismetMathLibrary.Normal` (- _impactpoint (`SceneComponent.GetSocketLocation` (`self.CharacterWeaponMesh`) (`self.MuzzleSocket`)))))
  ;[1 1 1] Bullet Hit
  (`/Engine/EditorBlueprintResources/StandardMacros.IsValid` _hitactor
    (:`Is Valid`
      (`GameplayStatics.SpawnEmitterAtLocation` _particle _impactpoint (`KismetMathLibrary.MakeRotator` (.roll _returnvalue) (+ (.pitch _returnvalue) -90.0) (.yaw _returnvalue)))
      (`GameplayStatics.SpawnDecalAttached` _decal _decalsize _hitcomponent _hitbonename _impactpoint _decalrotation "KeepWorldPosition" 40.0)
      (`GameplayStatics.SpawnSoundAtLocation` _soundhit _impactpoint (struct) 1.0 1.0 0.0 null null)
      (message `/Game/Blueprints/Weapon/BP_WeaponInterface.WeaponMakeNoise` (`self.OwnerCharacter`) (`.HitLoudness_13_76B107EF45518C88B410BA9A807311A0` (break `/Game/Blueprints/Weapon/Structures/Struct_Weapon/Struct_Weapon_Damage` (`.Damage_8_93B86D544DB6A894C92897AA97600886` (break `/Game/Blueprints/Weapon/Structures/Struct_Weapon/Struct_Weapon` (`self.WeaponStruct`))))) _impactpoint (`self.OwnerCharacter`))
      (`GameplayStatics.ApplyPointDamage` _hitactor (select `bool` (`.UseBulletProjectile_1_63FC76DA40FF1A0AC334AFBB37AAC0B5` (break `/Game/Blueprints/Weapon/Structures/Struct_Weapon/Struct_Weapon_Bullet` _bulletprojectile)) :`false` _basedamage :`true` `DamageUpdate(ric)`) (10.0 10.0 10.0) Hit null (`self.OwnerCharacter`) _damagetype_2) ; Send More information about damage for damage reciever than apply damage
      (message `/Game/Blueprints/Weapon/BP_WeaponInterface.CustomDamageDirection` _hitactor _returnvalue_2 _hitbonename _damagetype)
      (if (`SceneComponent.IsSimulatingPhysics` _hitcomponent _hitbonename)
        (`PrimitiveComponent.AddImpulse` _hitcomponent (* _returnvalue_2 (`KismetMathLibrary.SelectFloat` (`.DamageImpulse` (defaults `/Game/Blueprints/Weapon/BP_Weapon` _damagetype)) 15.0 (`KismetMathLibrary.ClassIsChildOf` (`GameplayStatics.GetObjectClass` _hitactor) "/Game/Blueprints/Car/BP_PawnCar.BP_PawnCar_C"))) _hitbonename true))
      (if (`.UseRadialDamage_3_4609DC0244CD6964F7DD2EBD7C0CF19A` (break `/Game/Blueprints/Weapon/Structures/Struct_Weapon/Struct_Weapon_Damage` (`.Damage_8_93B86D544DB6A894C92897AA97600886` (break `/Game/Blueprints/Weapon/Structures/Struct_Weapon/Struct_Weapon` (`self.WeaponStruct`)))))
        _))))

(event `SpreadingDecrease`
  ;[1 1 1] Spreading
  (set `self.DegreesCurrent` (+ (`self.Degrees`) (`.Spreading_Increase_12_1E35C52A41FB81F3DCA7B3864737D8CD` (break `/Game/Blueprints/Weapon/Structures/Struct_Weapon/Struct_Weapon_Spreading` (`.Spreading_21_99892FAD48D8FDC516D29698A779D626` (break `/Game/Blueprints/Weapon/Structures/Struct_Weapon/Struct_Weapon` (`self.WeaponStruct`)))))))
  (set `self.ForTimer` 0.0)
  (bind _returnvalue (`KismetSystemLibrary.K2_SetTimerDelegate` (delegate `Spreading`) 0.03 true))
  (`KismetSystemLibrary.RetriggerableDelay` (`.Spreading_Decrease_Time_13_9841C9934AEB696412E1DCB9BB56BFBA` (break `/Game/Blueprints/Weapon/Structures/Struct_Weapon/Struct_Weapon_Spreading` (`.Spreading_21_99892FAD48D8FDC516D29698A779D626` (break `/Game/Blueprints/Weapon/Structures/Struct_Weapon/Struct_Weapon` (`self.WeaponStruct`))))))
  (`KismetSystemLibrary.K2_ClearAndInvalidateTimerHandle` _returnvalue)
  (set `self.Degrees` (`.SpreadingCone_Min_6_6DB4D1134726323399510D8AE3942C92` (break `/Game/Blueprints/Weapon/Structures/Struct_Weapon/Struct_Weapon_Spreading` (`.Spreading_21_99892FAD48D8FDC516D29698A779D626` (break `/Game/Blueprints/Weapon/Structures/Struct_Weapon/Struct_Weapon` (`self.WeaponStruct`)))))))

(event `Spreading`
  (bind ((`SpreadingCone_Min_6_6DB4D1134726323399510D8AE3942C92` _spreadingcone_min) (`SpreadingCone_Max_8_51BEC7E5450C6EBB73CE5EA53339EB14` _spreadingcone_max) (`Spreading_Decrease_Time_13_9841C9934AEB696412E1DCB9BB56BFBA` _spreading_decrease_time)) (break `/Game/Blueprints/Weapon/Structures/Struct_Weapon/Struct_Weapon_Spreading` (`.Spreading_21_99892FAD48D8FDC516D29698A779D626` (break `/Game/Blueprints/Weapon/Structures/Struct_Weapon/Struct_Weapon` (`self.WeaponStruct`)))))
  ;[1 1 1] Spreading
  (set `self.Degrees` (`KismetMathLibrary.FClamp` (`KismetMathLibrary.Lerp` (`self.DegreesCurrent`) 0.15 (+ (/ (`self.ForTimer`) _spreading_decrease_time) 0.06)) _spreadingcone_min _spreadingcone_max))
  (set `self.ForTimer` (+ (`self.ForTimer`) 0.03)))

(fn `BulletDirection`
  (returns (Start :type "Vector Structure") (End :type "Vector Structure"))
  (bind _degrees (`self.Degrees`))
  (bind (_bulletstartlocation _shootdirection) (message `/Game/Blueprints/Weapon/BP_WeaponInterface.GetShootDirection` (`self.OwnerCharacter`))) ; Bullet Start location = Player camera world position\nShoot Direction = Player camera forward vector
  (return (+ _bulletstartlocation (* _shootdirection (`self.BulletTraceStartPos`))) (+ _bulletstartlocation (* (`KismetMathLibrary.RandomUnitVectorInEllipticalConeInDegrees` _shootdirection _degrees _degrees) 20000.0))))

(fn `BulletTrace`
  (params (MuzzleLoc :type "Vector Structure") (MuzzleRot :type "Rotator Structure"))
  (bind (_start _end) (`self.BulletDirection`))
  (bind (_outhit _returnvalue) (`KismetSystemLibrary.LineTraceSingleForObjects` (+ MuzzleLoc (* (`KismetMathLibrary.Conv_RotatorToVector` MuzzleRot) -50.0)) MuzzleLoc (`|MakeArray` "ObjectTypeQuery1" "ObjectTypeQuery2" "ObjectTypeQuery5" "ObjectTypeQuery6" "ObjectTypeQuery8" "ObjectTypeQuery4" :!type "EObjectTypeQuery Enum") false (`|MakeArray` (`self.OwnerCharacter`))))
  (if _returnvalue
    (`self.SpreadingDecrease`)
    (`self.BulletHit` _outhit)
    (else
      (bind _outhit_2 (`KismetSystemLibrary.LineTraceSingleForObjects` _start _end (`|MakeArray` "ObjectTypeQuery1" "ObjectTypeQuery2" "ObjectTypeQuery5" "ObjectTypeQuery6" "ObjectTypeQuery8" "ObjectTypeQuery4" :!type "EObjectTypeQuery Enum") true (`|MakeArray` (`self.OwnerCharacter`))))
      (`self.SpreadingDecrease`)
      (`self.BulletHit` _outhit_2))))

(fn `CheckWeaponCollision`
  (params (MuzzleLoc :type "Vector Structure") (MuzzleRot :type "Rotator Structure"))
  (returns (BulletStartLocation :type "Vector Structure"))
  (return (0.0 0.0 0.0)))