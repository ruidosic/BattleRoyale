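; Pickup item base Blueprint that registers itself with the player's interaction component and shows a floating 3D label when approached.
; Trigger overlap adds or removes the item in the player's InteractionItemArray, reached through GetComponentsMessage, and toggles the label if Active.
; Timelines scale the text in and out, while a looping timer rotates it toward the player camera until hidden.
; The pickup action itself is not implemented here.
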(event `self.Trigger.OnComponentBeginOverlap`
  (params (OverlappedComponent :type "PrimitiveComponent Object Reference") (OtherActor :type "Actor Object Reference") (OtherComp :type "PrimitiveComponent Object Reference") (OtherBodyIndex :type Integer) (bFromSweep :type Boolean) (SweepResult :type "HitResult Structure (by ref)"))
  (if (`self.IsPlayer` OtherActor)
    (bind _output_get (set `self.Character` OtherActor))
    (bind (_hud _inventory _interaction) (message `/Game/Blueprints/Pawn/BPI_StatusInterface.GetComponents` _output_get))
    (set `/Game/Blueprints/Pawn/Components/BP_Interaction.IsTriggerOverlap` true _interaction)
    (set `self.TriggerOverlap` true)
    (bind (_hud_2 _inventory_2 _interaction_2) (message `/Game/Blueprints/Pawn/BPI_StatusInterface.GetComponents` (`self.Character`)))
    (bind _interactionitem_array (`/Game/Blueprints/Pawn/Components/BP_Interaction.InteractionItem_Array` _interaction_2))
    (`KismetArrayLibrary.Array_AddUnique` _interactionitem_array self)
    (bind (_hud_3 _inventory_3 _interaction_3) (message `/Game/Blueprints/Pawn/BPI_StatusInterface.GetComponents` (`self.Character`)))
    (set `/Game/Blueprints/Pawn/Components/BP_Interaction.InteractionItem_Array` _interactionitem_array _interaction_3)
    (if (`self.Active`)
      (`self.TextActivate`))))

(event `self.Trigger.OnComponentEndOverlap`
  (params (OverlappedComponent :type "PrimitiveComponent Object Reference") (OtherActor :type "Actor Object Reference") (OtherComp :type "PrimitiveComponent Object Reference") (OtherBodyIndex :type Integer))
  (if (`self.IsPlayer` OtherActor)
    (bind _output_get (set `self.Character` OtherActor))
    (bind (_hud _inventory _interaction) (message `/Game/Blueprints/Pawn/BPI_StatusInterface.GetComponents` _output_get))
    (bind _interactionitem_array (`/Game/Blueprints/Pawn/Components/BP_Interaction.InteractionItem_Array` _interaction))
    (`KismetArrayLibrary.Array_RemoveItem` _interactionitem_array self)
    (bind (_hud_2 _inventory_2 _interaction_2) (message `/Game/Blueprints/Pawn/BPI_StatusInterface.GetComponents` (`self.Character`)))
    (set `/Game/Blueprints/Pawn/Components/BP_Interaction.InteractionItem_Array` _interactionitem_array _interaction_2)
    (if (`self.Active`)
      (`self.TextDeactivate`))))

(event `TextActivate`
  (bind _item3dtext (`self.Item3dText`))
  (bind (_hud _inventory _interaction _playercamera) (message `/Game/Blueprints/Pawn/BPI_StatusInterface.GetComponents` (`self.Character`)))
  (bind _returnvalue (`KismetSystemLibrary.K2_SetTimerDelegate` (delegate `TextLookAt`) 0.01 true))
  (set `self.TextLookAtTimer` _returnvalue)
  (`SceneComponent.SetVisibility` _item3dtext true false)
  (set `self.CurrentTextScale` (`SceneComponent.K2_GetComponentScale` _item3dtext))
  (bind (_direction _alpha) (`Timeline|TextScaleIncrease` :!via `PlayFromStart`)
    (:`Update`
      (`SceneComponent.SetWorldScale3D` (`self.Item3dText`) (`KismetMathLibrary.VLerp` (`self.CurrentTextScale`) (0.7 0.7 0.7) _alpha)))))

(event `TextDeactivate`
  (set `self.CurrentTextScale` (`SceneComponent.K2_GetComponentScale` (`self.Item3dText`)))
  (bind (_direction _alpha) (`Timeline|TextScaleDeincrease` :!via `PlayFromStart`)
    (:`Update`
      (`SceneComponent.SetWorldScale3D` (`self.Item3dText`) (`KismetMathLibrary.VLerp` (`self.CurrentTextScale`) (0.0 0.0 0.0) _alpha)))
    (:`Finished`
      (`KismetSystemLibrary.K2_ClearAndInvalidateTimerHandle` (`self.TextLookAtTimer`))
      (`SceneComponent.SetVisibility` (`self.Item3dText`) false false))))

(event `TextLookAt`
  (`SceneComponent.K2_SetWorldRotation` (`self.Item3dText`) (`KismetMathLibrary.Conv_VectorToRotator` (- (`SceneComponent.K2_GetComponentLocation` (stale `TextActivate` _playercamera)) (`SceneComponent.K2_GetComponentLocation` (`self.Item3dText`)))) false false))

(fn `IsPlayer`
  (params (Actor :type "Object Object Reference"))
  (returns (IsPlayer :type Boolean))
  (return (== Actor (`GameplayStatics.GetPlayerPawn` 0))))

(fn `UserConstructionScript`)